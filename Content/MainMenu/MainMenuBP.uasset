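; Main menu Blueprint that loads the StatSave slot on BeginPlay and chooses which UI to open.
; With HasSave set, it copies stats and slime cores to MyPlayer, shows MainUI, spawns red, blue and green enemies, and writes them with their images into StageList.
; Without HasSave it shows CreateUser.
; A failed load cast stops startup, as the HasSave reset branch is unconnected.
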(event EventBeginPlay
  (bind _outactors (Actor|GetAllActorsOfClass "/Game/Characters/Actors/MyPlayer.MyPlayer_C"))
  (Variables|Default|SetPlayerRef (Utilities|Array|Get(acopy) _outactors))
  (bind _returnvalue (SaveGame|CreateSaveGameObject "/Game/Characters/StatSave.StatSave_C"))
  (bind _asstat_save (Utilities|Casting|CastToStatSave _returnvalue))
  (bind _output_get (Variables|Default|SetSaveGame _asstat_save))
  (bind _returnvalue_2 (SaveGame|LoadGamefromSlot (Variables|/Game/Characters/StatSave.StatSave_C|GetSaveSlotName _output_get) (Variables|/Game/Characters/StatSave.StatSave_C|GetUserIndex _output_get)))
  (bind _asstat_save_2 (Utilities|Casting|CastToStatSave _returnvalue_2))
  (bind _output_get_2 (Variables|Default|SetSaveGame _asstat_save_2))
  (if (Variables|/Game/Characters/StatSave.StatSave_C|GetHasSave? _output_get_2)
    (CallFunction|LoadStatsandInv)
    (bind _returnvalue_3 (UserInterface|CreateWidget "/Game/UI/MainUI.MainUI_C" (Game|GetPlayerController 0)))
    (UserInterface|Viewport|AddtoViewport _returnvalue_3 0)
    (CallFunction|CreateEnemies)
    (CallFunction|SetStages)
    (else
      (bind _returnvalue_4 (UserInterface|CreateWidget "/Game/UI/CreateUser.CreateUser_C" (Game|GetPlayerController 0)))
      (UserInterface|Viewport|AddtoViewport _returnvalue_4 0))))

(fn ConstructionScript)

(fn CreateEnemies
  (bind _returnvalue (Game|SpawnActorfromClass "/Game/Characters/Actors/Enemy_Red.Enemy_Red_C" (Math|Transform|MakeTransform "0, 0, 0" "0, 0, 0" "1,1,1") "AlwaysSpawn" 0 0.0 0.0 0.0 0.0))
  (Variables|Default|SetRedEnemy _returnvalue)
  (bind _returnvalue_2 (Game|SpawnActorfromClass "/Game/Characters/Actors/Enemy_Blue.Enemy_Blue_C" (Math|Transform|MakeTransform "0, 0, 0" "0, 0, 0" "1,1,1") "AlwaysSpawn" 0 0.0 0.0 0.0 0.0))
  (Variables|Default|SetBlueEnemy _returnvalue_2)
  (bind _returnvalue_3 (Game|SpawnActorfromClass "/Game/Characters/Actors/Enemy_Green.Enemy_Green_C" (Math|Transform|MakeTransform "0, 0, 0" "0, 0, 0" "1,1,1") "AlwaysSpawn" 0 0.0 0.0 0.0 0.0))
  (Variables|Default|SetGreenEnemy _returnvalue_3))

(fn SetStages
  (Utilities|Array|SetArrayElem (Utilities|Struct|BreakStageList (Variables|Default|GetStageList)) 0 (Utilities|Struct|MakeEnemyList (Utilities|Array|MakeArray (Variables|Default|GetRedEnemy) (Variables|Default|GetBlueEnemy) (Variables|Default|GetGreenEnemy)) (Utilities|Array|MakeArray (Variables|Default|GetMatRed) (Variables|Default|GetMatBlue) (Variables|Default|GetMatGreen)))))

(fn LoadStatsandInv
  (bind _playerref (Variables|Default|GetPlayerRef))
  (bind _savegame (Variables|Default|GetSaveGame))
  (bind _slimecoresinv (Variables|/Game/Characters/Actors/MyCharacterClass.MyCharacterClass_C|GetSlimeCoresInv _playerref))
  (bind _slimecoresequipped (Variables|/Game/Characters/Actors/MyCharacterClass.MyCharacterClass_C|GetSlimeCoresEquipped _playerref))
  (Variables|/Game/Characters/Actors/MyCharacterClass.MyCharacterClass_C|SetStats _playerref (Variables|/Game/Characters/StatSave.StatSave_C|GetStats _savegame))
  (Utilities|Array|Clear _slimecoresequipped)
  (for _array_element (Variables|/Game/Characters/StatSave.StatSave_C|GetCores _savegame)
    (Utilities|Array|Add _slimecoresequipped _array_element))
  (Utilities|Array|Clear _slimecoresinv)
  (for _array_element_2 (Variables|/Game/Characters/StatSave.StatSave_C|GetInventory _savegame)
    (Utilities|Array|Add _slimecoresinv _array_element_2)))